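; Tank pawn Blueprint that sets up the barrel reference and drives the player's orbiting aim view.
; On BeginPlay it passes the GunBarrel component to SetTankBarrelRef.
; Aim axis inputs yaw the Gimbal and pitch the SpringArm separately in local space, scaled by delta time for a frame-rate-independent turn speed.
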(event EventBeginPlay
  (Class|Tank|SetTankBarrelRef (Variables|Default|GetGunBarrel)))

(event Input|AxisEvents|InputAxisAim_Azimuth
  (params (AxisValue :type Float%20%28single-precision%29))
  (Transformation|AddLocalRotation (Variables|Default|GetGimbal) (Math|Rotator|MakeRotator 0.0 0.0 (* AxisValue (Utilities|Time|GetWorldDeltaSeconds) 1e+02)) false false))

(event Input|AxisEvents|InputAxisAim_Elevation
  (params (AxisValue :type Float%20%28single-precision%29))
  (Transformation|AddLocalRotation (Variables|Default|GetSpringArm) (Math|Rotator|MakeRotator 0.0 (* AxisValue (Utilities|Time|GetWorldDeltaSeconds) 1e+02) 0.0) false false))

(fn ConstructionScript)